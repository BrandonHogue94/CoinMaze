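; 30Coin_BP is a coin-gated door that ends the game once the top-down character has collected enough coins.
; On TriggerDoor overlap it compares the character's CoinCount against RequiredCoins30.
; If met, it destroys itself, calls RemoveCoin30 on the character and shows the EndGame widget.
; Otherwise it prints a prompt to collect more coins.
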(event OnComponentBeginOverlap(TriggerDoor)
  (params (OverlappedComponent :type Primitive%20Component%20Object%20Reference) (OtherActor :type Actor%20Object%20Reference) (OtherComp :type Primitive%20Component%20Object%20Reference) (OtherBodyIndex :type Integer) (bFromSweep :type Boolean) (SweepResult :type Hit%20Result%20Structure%20%28by%20ref%29))
  (bind _asbp_top_down_character (Utilities|Casting|CastToBP_TopDownCharacter OtherActor))
  (if (>= (Variables|/Game/TopDown/Blueprints/BP_TopDownCharacter.BP_TopDownCharacter_C|GetCoin_Count _asbp_top_down_character) (Variables|Default|GetRequiredCoins30))
    (Actor|DestroyActor)
    (bind _asbp_top_down_character_2 (Utilities|Casting|CastToBP_TopDownCharacter OtherActor))
    (Default|RemoveCoin30 _asbp_top_down_character_2)
    (bind _returnvalue (UserInterface|CreateWidget "/Game/UI/EndGame.EndGame_C" (Game|GetPlayerController 0)))
    (UserInterface|Viewport|AddtoViewport _returnvalue 0)
    (else
      (Development|PrintString "Collect More Coins!"))))

(fn ConstructionScript)